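; Squeenk creature actor that grows from an embryo, then wanders in random steps within a radius of the world origin.
; Collider overlaps between non-busy grown creatures interrupt movement to breed with Squeenks, fight Beasts or kill Tentacles.
; Breeding posts midpoint and parents to GameManagerBP; Beast fights roll randomly weighted by Power.
; Comparing X+Y positions picks which side posts or rolls, while Delay loops poll for busy slots and fight results.
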(event OnComponentBeginOverlap(Collider)
  (params (OverlappedComponent :type Primitive%20Component%20Object%20Reference) (OtherActor :type Actor%20Object%20Reference) (OtherComp :type Primitive%20Component%20Object%20Reference) (OtherBodyIndex :type Integer) (bFromSweep :type Boolean) (SweepResult :type Hit%20Result%20Structure%20%28by%20ref%29))
  (bind _squeenk (Variables|Default|GetSqueenk))
  (bind _squeenk_2 (Variables|Default|GetSqueenk))
  (bind _rootcomponent (Variables|/Script/Engine.Actor|GetRootComponent OtherActor))
  (bind _squeenk_3 (Variables|Default|GetSqueenk))
  (bind _power (Variables|Default|GetPower))
  (bind _squeenk_4 (Variables|Default|GetSqueenk))
  (bind _returnvalue (Transformation|GetWorldLocation _squeenk_4))
  (bind _returnvalue_2 (Math|Vector|GetForwardVector _squeenk))
  (bind _returnvalue_3 (Transformation|GetWorldLocation _squeenk_2))
  (bind _returnvalue_4 (Transformation|GetWorldLocation _squeenk))
  (bind _returnvalue_5 (Transformation|GetWorldLocation _squeenk_3))
  (bind _returnvalue_6 (Transformation|GetWorldLocation _rootcomponent))
  (bind _returnvalue_7 (Math|Vector|GetForwardVector _squeenk_3))
  (bind _returnvalue_8 (Transformation|GetWorldLocation _squeenk_3))
  (bind _returnvalue_9 (Transformation|GetWorldLocation _squeenk_4))
  (bind _returnvalue_10 (Math|Vector|GetUnitDirection(Vector) _returnvalue_6 _returnvalue_5))
  (Variables|Default|Setcollided true)
  (bind _assqueenk_bp (Utilities|Casting|CastToSqueenkBP OtherActor)
    (:then
      (if (Math|Boolean|ANDBoolean (Actor|ActorHasTag OtherActor "Squeenk") (not (Variables|SqueenkBP_C|Getbusy _assqueenk_bp)) (not (Variables|Default|Getbusy)) (>= (Variables|Default|Getembryo) 1.0) (>= (Variables|SqueenkBP_C|Getembryo _assqueenk_bp) 1.0)) :!label _label
        (bind _output_get (Variables|Default|Settarget _assqueenk_bp))
        (Utilities|FlowControl|Delay 0.0)
        (Variables|Default|Setbusy true)
        (Utilities|FlowControl|Sequence
          (:then_0
            (goto _label_3 Stop))
          (:then_1
            (goto _label_6 Stop))
          (:then_2
            (Components|MoveComponentTo _squeenk_3 _returnvalue_5 (Math|Conversions|RotationFromXVector (Math|Vector|MakeVector (* (.y _returnvalue_10) 1.0) (* (.x _returnvalue_10) -1.0) 0.0)) false false 0.5 true)
            (Components|Animation|PlayAnimation _squeenk_3 "/Game/Beings/Squeenk/Squeenk_Anim_Squeenk_mesh_create.Squeenk_Anim_Squeenk_mesh_create" false)
            (bind _returnvalue_11 (Actor|GetActorOfClass "/Game/Blueprints/GameManagerBP.GameManagerBP_C"))
            (Math|Float|CompareFloat (+ (.x _returnvalue_8) (.y _returnvalue_8)) (+ (.x (Transformation|GetWorldLocation (Variables|/Script/Engine.Actor|GetRootComponent _output_get))) (.y (Transformation|GetWorldLocation (Variables|/Script/Engine.Actor|GetRootComponent _output_get))))
              (:>
                (if (Math|Vector|Equal(Vector) (Variables|/Game/Blueprints/GameManagerBP.GameManagerBP_C|GetnewSqueenkLocation _returnvalue_11) "-1000.000000,-1000.000000,-1000.000000" 0.0001) :!label _label_2
                  (Variables|/Game/Blueprints/GameManagerBP.GameManagerBP_C|SetnewSqueenkLocation _returnvalue_11 (/ (+ (Transformation|GetWorldLocation _rootcomponent) (Transformation|GetWorldLocation _squeenk_3)) 2.0))
                  (Variables|/Game/Blueprints/GameManagerBP.GameManagerBP_C|SetnewSqueenkParent _returnvalue_11 self)
                  (Variables|/Game/Blueprints/GameManagerBP.GameManagerBP_C|SetnewSqueenkOtherParent _returnvalue_11 _output_get)
                  (else
                    (Utilities|FlowControl|Delay 0.01)
                    (goto _label_2))))
              (:<
                _))
            (Utilities|FlowControl|Delay 6.0)
            (Variables|Default|Setcollided false)
            (Variables|Default|SetdontKeepBusy true)
            (Components|Animation|PlayAnimation _squeenk_3 "/Game/Beings/Squeenk/Squeenk_Anim_Squeenk_mesh_walk.Squeenk_Anim_Squeenk_mesh_walk" true)
            (Variables|Default|SetrandomRotation (+ (.yaw (Math|Conversions|RotationFromXVector (Math|Vector|MakeVector (* (.y _returnvalue_7) 1.0) (* (.x _returnvalue_7) -1.0) 0.0))) (Math|Random|RandomFloatinRange 1.6e+02 2e+02)))
            (Components|MoveComponentTo _squeenk _returnvalue_4 (Math|Rotator|MakeRotator 0.0 0.0 (stale _output_get_3)) false false 0.3 true :!label _label_3)
            (if (and (Variables|Default|Getbusy) (Variables|Default|Getcollided))
              (if (Variables|Default|GetdontKeepBusy)
                (bind _output_get_2 (Variables|Default|SetrandomLocation (+ _returnvalue_4 (* (Math|Vector|MakeVector (* (.y _returnvalue_2) 1.0) (* (.x _returnvalue_2) -1.0) 0.0) 8e+02)) :!label _label_4))
                (Math|Float|CompareFloat (Math|Vector|Distance(Vector) "0, 0, 0" _output_get_2) 2.3e+03
                  (:>
                    (bind _output_get_3 (Variables|Default|SetrandomRotation (Math|Random|RandomFloatinRange 0.0 3.6e+02) :!label _label_5))
                    (goto _label_3))
                  (:<
                    (Components|MoveComponentTo _squeenk _output_get_2 (Math|Rotator|MakeRotator 0.0 0.0 _output_get_3) false false 1.0 false :!label _label_6)
                    (if (and (Variables|Default|Getbusy) (Variables|Default|Getcollided))
                      (if (Variables|Default|GetdontKeepBusy)
                        (Variables|Default|Setbusy false :!label _label_7)
                        (Variables|Default|SetdontKeepBusy false)
                        (goto _label_5))
                      (else
                        (goto _label_7))))))
              (else
                (goto _label_4)))))
        (else
          (Utilities|FlowControl|Delay 0.2)
          (if (Class|PrimitiveComponent|IsOverlappingComponent (Variables|Default|GetCollider))
            (goto _label)))))
    (:CastFailed
      (bind _asbeast_bp (Utilities|Casting|CastToBeastBP OtherActor)
        (:then
          (if (Math|Boolean|ANDBoolean (Actor|ActorHasTag OtherActor "Beast") (not (Variables|/Game/Blueprints/BeastBP.BeastBP_C|Getbusy _asbeast_bp)) (not (Variables|Default|Getbusy)) (>= (Variables|Default|Getembryo) 1.0) (>= (Variables|/Game/Blueprints/BeastBP.BeastBP_C|Getembryo _asbeast_bp) 1.0)) :!label _label_8
            (bind _output_get_4 (Variables|Default|Settarget _asbeast_bp))
            (Utilities|FlowControl|Delay 0.0)
            (Variables|Default|Setbusy true)
            (Utilities|FlowControl|Sequence
              (:then_0
                (goto _label_3 Stop))
              (:then_1
                (goto _label_6 Stop))
              (:then_2
                (Math|Float|CompareFloat (+ (.x _returnvalue) (.y _returnvalue)) (+ (.x (Transformation|GetWorldLocation (Variables|/Script/Engine.Actor|GetRootComponent _output_get_4))) (.y (Transformation|GetWorldLocation (Variables|/Script/Engine.Actor|GetRootComponent _output_get_4))))
                  (:>
                    (Math|Integer|CompareInt (Math|Random|RandomIntegerinRange 1 (+ (Variables|/Game/Blueprints/BeastBP.BeastBP_C|Getpower _asbeast_bp) _power)) _power
                      (:>
                        (Variables|/Game/Blueprints/BeastBP.BeastBP_C|SetkillCommand _asbeast_bp true))
                      (:==
                        (Variables|Default|SetkillCommand true :!label _label_9)
                        (Components|MoveComponentTo _squeenk_4 _returnvalue_9 (Math|Conversions|RotationFromXVector (Math|Vector|MakeVector (* (.y (Math|Vector|GetUnitDirection(Vector) (Transformation|GetWorldLocation (Variables|/Script/Engine.Actor|GetRootComponent _output_get_4)) _returnvalue_9)) 1.0) (* (.x (Math|Vector|GetUnitDirection(Vector) (Transformation|GetWorldLocation (Variables|/Script/Engine.Actor|GetRootComponent _output_get_4)) _returnvalue_9)) -1.0) 0.0)) false false 0.5 true :!label _label_10)
                        (Components|Animation|PlayAnimation _squeenk_4 "/Game/Beings/Squeenk/Squeenk_Anim_Squeenk_mesh_attack.Squeenk_Anim_Squeenk_mesh_attack" false)
                        (Audio|PlaySound2D "/Game/Audio/Squeenk_attack.Squeenk_attack" 1.0 1.0 0.0 0 0)
                        (Utilities|FlowControl|Delay 0.5)
                        (bind _returnvalue_12 (Effects|SpawnEmitteratLocation "/Game/Effects/Death.Death" (Math|Vector|MakeVector (.x (Transformation|GetActorLocation _output_get_4)) (.y (Transformation|GetActorLocation _output_get_4)) (.z (Transformation|GetActorLocation _output_get_4)))))
                        (Effects|Components|ParticleSystem|SetColorParameter _returnvalue_12 "color" "(R=0.041667,G=0.021791,B=0.041134,A=1.000000)")
                        (Components|MoveComponentTo _squeenk_4 (Math|Vector|MakeVector (.x (Transformation|GetActorLocation _output_get_4)) (.y (Transformation|GetActorLocation _output_get_4)) -2e+01) (Math|Conversions|RotationFromXVector (Math|Vector|MakeVector (* (.y (Math|Vector|GetUnitDirection(Vector) (Transformation|GetWorldLocation (Variables|/Script/Engine.Actor|GetRootComponent _output_get_4)) _returnvalue_9)) 1.0) (* (.x (Math|Vector|GetUnitDirection(Vector) (Transformation|GetWorldLocation (Variables|/Script/Engine.Actor|GetRootComponent _output_get_4)) _returnvalue_9)) -1.0) 0.0)) false false 0.5 true)
                        (Audio|PlaySound2D "/Game/Audio/Death.Death" 1.0 1.0 0.0 0 0)
                        (Actor|DestroyActor _output_get_4)
                        (Variables|Default|Setcollided false)
                        (Variables|Default|SetdontKeepBusy true)
                        (Variables|Default|SetkillCommand false)
                        (Components|Animation|PlayAnimation _squeenk_4 "/Game/Beings/Squeenk/Squeenk_Anim_Squeenk_mesh_walk.Squeenk_Anim_Squeenk_mesh_walk" true)
                        (goto _label_5))
                      (:<
                        (goto _label_9))))
                  (:<
                    (Utilities|FlowControl|Delay 0.01 :!label _label_11)
                    (if (Variables|Default|GetkillCommand)
                      (goto _label_10)
                      (elif (not (Variables|/Game/Blueprints/BeastBP.BeastBP_C|GetkillCommand _asbeast_bp))
                        (goto _label_11)))))))
            (else
              (Utilities|FlowControl|Delay 0.2)
              (if (Class|PrimitiveComponent|IsOverlappingComponent (Variables|Default|GetCollider))
                (goto _label_8)))))
        (:CastFailed
          (bind _astentacle_bp (Utilities|Casting|CastToTentacleBP OtherActor))
          (if (Math|Boolean|ANDBoolean (Actor|ActorHasTag OtherActor "Tentacle") (not (Variables|/Game/Blueprints/TentacleBP.TentacleBP_C|Getembryo _astentacle_bp)) (>= (Variables|Default|Getembryo) 1.0) (not (Variables|/Game/Blueprints/TentacleBP.TentacleBP_C|Getbusy _astentacle_bp)) (not (Variables|Default|Getbusy))) :!label _label_12
            (bind _output_get_5 (Variables|Default|Settarget _astentacle_bp))
            (Utilities|FlowControl|Delay 0.0)
            (Variables|Default|Setbusy true)
            (Variables|/Game/Blueprints/TentacleBP.TentacleBP_C|Setbusy _astentacle_bp true)
            (Utilities|FlowControl|Sequence
              (:then_0
                (goto _label_3 Stop))
              (:then_1
                (goto _label_6 Stop))
              (:then_2
                (Components|MoveComponentTo _squeenk_2 _returnvalue_3 (Math|Conversions|RotationFromXVector (Math|Vector|MakeVector (* (.y (Math|Vector|GetUnitDirection(Vector) (Transformation|GetWorldLocation (Variables|/Script/Engine.Actor|GetRootComponent _output_get_5)) _returnvalue_3)) 1.0) (* (.x (Math|Vector|GetUnitDirection(Vector) (Transformation|GetWorldLocation (Variables|/Script/Engine.Actor|GetRootComponent _output_get_5)) _returnvalue_3)) -1.0) 0.0)) false false 0.5 true)
                (Components|Animation|PlayAnimation _squeenk_2 "/Game/Beings/Squeenk/Squeenk_Anim_Squeenk_mesh_attack.Squeenk_Anim_Squeenk_mesh_attack" false)
                (Audio|PlaySound2D "/Game/Audio/Squeenk_attack.Squeenk_attack" 1.0 1.0 0.0 0 0)
                (Utilities|FlowControl|Delay 0.5)
                (Variables|/Game/Blueprints/TentacleBP.TentacleBP_C|Setdeath _astentacle_bp true)
                (Components|MoveComponentTo _squeenk_2 (Math|Vector|MakeVector (.x (Transformation|GetWorldLocation (Variables|/Script/Engine.Actor|GetRootComponent _output_get_5))) (.y (Transformation|GetWorldLocation (Variables|/Script/Engine.Actor|GetRootComponent _output_get_5))) -2e+01) (Math|Conversions|RotationFromXVector (Math|Vector|MakeVector (* (.y (Math|Vector|GetUnitDirection(Vector) (Transformation|GetWorldLocation (Variables|/Script/Engine.Actor|GetRootComponent _output_get_5)) _returnvalue_3)) 1.0) (* (.x (Math|Vector|GetUnitDirection(Vector) (Transformation|GetWorldLocation (Variables|/Script/Engine.Actor|GetRootComponent _output_get_5)) _returnvalue_3)) -1.0) 0.0)) false false 0.5 true)
                (Variables|Default|Setcollided false)
                (Variables|Default|SetdontKeepBusy true)
                (Variables|Default|SetkillCommand false)
                (Components|Animation|PlayAnimation _squeenk_2 "/Game/Beings/Squeenk/Squeenk_Anim_Squeenk_mesh_walk.Squeenk_Anim_Squeenk_mesh_walk" true)
                (goto _label_5)))
            (else
              (Utilities|FlowControl|Delay 0.2)
              (if (Class|PrimitiveComponent|IsOverlappingComponent (Variables|Default|GetCollider))
                (goto _label_12)))))))))

(event EventBeginPlay
  (bind _squeenk (Variables|Default|GetSqueenk))
  (bind _returnvalue (Math|Vector|GetForwardVector _squeenk))
  (bind _returnvalue_2 (Transformation|GetWorldLocation _squeenk))
  (Math|Float|CompareFloat (Variables|Default|Getembryo) 1.0 :!label _label
    (:>
      _)
    (:==
      _)
    (:<
      (Transformation|SetActorScale3D (.scale (Math|Transform|Lerp(Transform) (Math|Transform|MakeTransform "0, 0, 0" "0, 0, 0" "0.000000,0.000000,0.000000") (Math|Transform|MakeTransform "0, 0, 0") (Variables|Default|Getembryo))))
      (Math|Float|CompareFloat (Variables|Default|Getembryo) 0.0
        (:>
          _)
        (:==
          (Utilities|FlowControl|Delay 2.1))
        (:<
          _))
      (Variables|Default|Setembryo (+ (Variables|Default|Getembryo) 0.035))
      (Utilities|FlowControl|Delay 0.1)
      (goto _label)))
  (Components|Animation|PlayAnimation _squeenk "/Game/Beings/Squeenk/Squeenk_Anim_Squeenk_mesh_walk.Squeenk_Anim_Squeenk_mesh_walk" true)
  (bind _output_get (Variables|Default|SetrandomRotation (Math|Random|RandomFloatinRange 0.0 3.6e+02) :!label _label_2))
  (Components|MoveComponentTo _squeenk _returnvalue_2 (Math|Rotator|MakeRotator 0.0 0.0 _output_get) false false 0.3 true)
  (if (and (Variables|Default|Getbusy) (Variables|Default|Getcollided))
    (if (Variables|Default|GetdontKeepBusy)
      (bind _output_get_2 (Variables|Default|SetrandomLocation (+ _returnvalue_2 (* (Math|Vector|MakeVector (* (.y _returnvalue) 1.0) (* (.x _returnvalue) -1.0) 0.0) 8e+02)) :!label _label_3))
      (Math|Float|CompareFloat (Math|Vector|Distance(Vector) "0, 0, 0" _output_get_2) 2.3e+03
        (:>
          (goto _label_2))
        (:<
          (Components|MoveComponentTo _squeenk _output_get_2 (Math|Rotator|MakeRotator 0.0 0.0 _output_get) false false 1.0 false)
          (if (and (Variables|Default|Getbusy) (Variables|Default|Getcollided))
            (if (Variables|Default|GetdontKeepBusy)
              (Variables|Default|Setbusy false :!label _label_4)
              (Variables|Default|SetdontKeepBusy false)
              (goto _label_2))
            (else
              (goto _label_4))))))
    (else
      (goto _label_3))))

(fn ConstructionScript)
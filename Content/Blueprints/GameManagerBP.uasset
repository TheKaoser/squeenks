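; Game manager for a three-faction survival match between Beasts, Squeenks and a tentacled Creature, covering menu, music, spawning and end screen.
; BeginPlay polls GameStarted, then spawns each faction at random points, rejection-sampled within a radius.
; Tick counts tagged actors to eliminate factions, ending the match when one remains.
; It also spawns offspring at requested locations (sentinel vector means none), with parent rays for Squeenks, and adds tentacles on a timer.
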(event EventBeginPlay
  (bind _winner (Variables|Default|Getwinner))
  (bind _returnvalue (UserInterface|CreateWidget "/Game/Blueprints/MenuBP.MenuBP_C"))
  (UserInterface|Viewport|AddtoViewport _returnvalue 0)
  (bind _returnvalue_2 (Audio|SpawnSound2D "/Game/Audio/Menu.Menu" 1.0 1.0 0.0 0 false false))
  (Utilities|FlowControl|Delay 0.2 :!label _label)
  (if (Variables|Default|GetgameStarted)
    (Components|DestroyComponent _returnvalue_2)
    (bind _returnvalue_3 (Audio|SpawnSound2D "/Game/Audio/In_game.In_game" 1.0 1.0 0.0 0 false false))
    (for _index (range 0 2)
      (bind _output_get (Variables|Default|SetrandomLocation (Math|Vector|MakeVector (Math|Random|RandomFloatinRange -2.4e+03 2.4e+03) (Math|Random|RandomFloatinRange -2.4e+03 2.4e+03) -2e+01) :!label _label_2))
      (Math|Float|CompareFloat (Math|Vector|Distance(Vector) "0, 0, 0" _output_get) 2.3e+03
        (:>
          (goto _label_2))
        (:<
          (Game|SpawnActorfromClass "/Game/Blueprints/SqueenkBP.SqueenkBP_C" (Math|Transform|MakeTransform _output_get (Math|Rotator|MakeRotator 0.0 0.0 (Math|Random|RandomFloatinRange 0.0 3.6e+02))) "DontSpawnIfColliding" 0 0))))
    (for _index_2 (range 0 1)
      (bind _output_get_2 (Variables|Default|SetrandomLocation (Math|Vector|MakeVector (Math|Random|RandomFloatinRange -2.4e+03 2.4e+03) (Math|Random|RandomFloatinRange -2.4e+03 2.4e+03) -6e+01) :!label _label_3))
      (Math|Float|CompareFloat (Math|Vector|Distance(Vector) "0, 0, 0" _output_get_2) 2.3e+03
        (:>
          (goto _label_3))
        (:<
          (Game|SpawnActorfromClass "/Game/Blueprints/BeastBP.BeastBP_C" (Math|Transform|MakeTransform _output_get_2 (Math|Rotator|MakeRotator 0.0 0.0 (Math|Random|RandomFloatinRange 0.0 3.6e+02))) "DontSpawnIfColliding" 0 0))))
    (for _index_3 (range 0 1)
      (bind _output_get_3 (Variables|Default|SetrandomLocation (Math|Vector|MakeVector (Math|Random|RandomFloatinRange -5e+02 5e+02) (Math|Random|RandomFloatinRange -5e+02 5e+02) -2.5e+02) :!label _label_4))
      (Math|Float|CompareFloat (Math|Vector|Distance(Vector) "0, 0, 0" _output_get_3) 2.3e+03
        (:>
          (goto _label_4))
        (:<
          (Game|SpawnActorfromClass "/Game/Blueprints/TentacleBP.TentacleBP_C" (Math|Transform|MakeTransform _output_get_3 (Math|Rotator|MakeRotator 0.0 0.0 (Math|Random|RandomFloatinRange 0.0 3.6e+02)) "0.700000,0.700000,0.700000") "DontSpawnIfColliding" 0 0))))
    (Utilities|Array|Add _winner "Beasts")
    (Utilities|Array|Add _winner "Squeenks")
    (Utilities|Array|Add _winner "Creature")
    (else
      (goto _label))))

(event EventTick
  (params (DeltaSeconds :type Float%20%28single-precision%29))
  (bind _members (Variables|Default|Getmembers))
  (bind _winner (Variables|Default|Getwinner))
  (bind _winner_2 (Variables|Default|Getwinner))
  (bind _members_2 (Variables|Default|Getmembers))
  (bind _winner_3 (Variables|Default|Getwinner))
  (bind _members_3 (Variables|Default|Getmembers))
  (bind _newsqueenkparent (Variables|Default|GetnewSqueenkParent))
  (bind _newsqueenkotherparent (Variables|Default|GetnewSqueenkOtherParent))
  (bind _returnvalue (Transformation|GetActorTransform _newsqueenkparent))
  (bind _returnvalue_2 (Transformation|GetActorTransform _newsqueenkotherparent))
  (if (not (Variables|Default|GetfinishedGame))
    (if (Variables|Default|GetgameStarted)
      (bind _outactors (Actor|GetAllActorswithTag "Beast"))
      (for (_array_element _array_index) _outactors
        (Utilities|Map|Add _members_3 _array_element _array_index))
      (if (== (Utilities|Map|Length _members_3) 0)
        (if (Utilities|Array|ContainsItem _winner "Beasts")
          (Utilities|Array|RemoveItem _winner "Beasts")
          (if (== (Utilities|Array|Length _winner) 1) :!label _label
            (bind _returnvalue_3 (UserInterface|CreateWidget "/Game/Blueprints/FinalScreenBP.FinalScreenBP_C"))
            (UserInterface|Viewport|AddtoViewport _returnvalue_3 0)
            (Components|DestroyComponent (stale EventBeginPlay _returnvalue_3))
            (Variables|Default|SetfinishedGame true)
            (bind _outactors_2 (Actor|GetAllActorswithTag "NonTentacle"))
            (for _array_element_2 _outactors_2
              (Actor|DestroyActor _array_element_2))
            (bind _outactors_3 (Actor|GetAllActorswithTag "Tentacle"))
            (for _array_element_3 _outactors_3
              (Actor|DestroyActor _array_element_3)
              (bind _outactors_4 (Actor|GetAllActorswithTag "Ray"))
              (for _array_element_4 _outactors_4
                (Actor|DestroyActor _array_element_4))))
          (else
            (bind _outactors_5 (Actor|GetAllActorswithTag "Squeenk" :!label _label_2))
            (for (_array_element_5 _array_index_2) _outactors_5
              (Utilities|Map|Add _members _array_element_5 _array_index_2))
            (if (== (Utilities|Map|Length _members) 0)
              (if (Utilities|Array|ContainsItem _winner_2 "Squeenks")
                (Utilities|Array|RemoveItem _winner_2 "Squeenks")
                (goto _label)
                (else
                  _))
              (else
                (Utilities|Map|Clear _members)))
            (if (Math|Vector|NotEqual(Vector) (Variables|Default|GetnewSqueenkLocation) "-1000.000000,-1000.000000,-1000.000000" 0.0001)
              (bind _returnvalue_4 (Game|SpawnActorfromClass "/Game/Blueprints/SqueenkBP.SqueenkBP_C" (Math|Transform|MakeTransform (Variables|Default|GetnewSqueenkLocation) (Math|Rotator|MakeRotator 0.0 0.0 (Math|Random|RandomFloatinRange 0.0 3.6e+02))) "DontSpawnIfColliding" 0 0))
              (Variables|Default|SetnewSqueenkLocation "-1000.000000,-1000.000000,-1000.000000")
              (bind _returnvalue_5 (Game|SpawnActorfromClass "/Game/Blueprints/SqueenkRayBP.SqueenkRayBP_C" (Math|Transform|MakeTransform (+ (.location _returnvalue) "0.000000, 0,230.000000") (.rotation _returnvalue) "1,1,1") "Undefined" 0 0))
              (Effects|Components|ParticleSystem|SetActorParameter (Variables|/Game/Blueprints/SqueenkRayBP.SqueenkRayBP_C|GetSqueenkRay _returnvalue_5) "Target" _returnvalue_4)
              (bind _returnvalue_6 (Game|SpawnActorfromClass "/Game/Blueprints/SqueenkRayBP.SqueenkRayBP_C" (Math|Transform|MakeTransform (+ (.location _returnvalue_2) "0.000000, 0,230.000000") (.rotation _returnvalue_2) "1,1,1") "Undefined" 0 0))
              (Effects|Components|ParticleSystem|SetActorParameter (Variables|/Game/Blueprints/SqueenkRayBP.SqueenkRayBP_C|GetSqueenkRay _returnvalue_6) "Target" _returnvalue_4)
              (Actor|SetLifeSpan _returnvalue_6 5.6)
              (Audio|PlaySound2D "/Game/Audio/Squeenk_create.Squeenk_create" 1.0 1.0 0.0 0 0)
              (elif (Math|Vector|NotEqual(Vector) (Variables|Default|GetnewBeastLocation) "-1000.000000,-1000.000000,-1000.000000" 0.0001)
                (Game|SpawnActorfromClass "/Game/Blueprints/BeastBP.BeastBP_C" (Math|Transform|MakeTransform (Variables|Default|GetnewBeastLocation) (Math|Rotator|MakeRotator 0.0 0.0 (Math|Random|RandomFloatinRange 0.0 3.6e+02))) "DontSpawnIfColliding" 0 0)
                (Effects|SpawnEmitteratLocation "/Game/Effects/Smoke.Smoke" (Variables|Default|GetnewBeastLocation))
                (Variables|Default|SetnewBeastLocation "-1000.000000,-1000.000000,-1000.000000")
                (Audio|PlaySound2D "/Game/Audio/Beast_create.Beast_create" 1.0 1.0 0.0 0 0)
                (else
                  (bind _output_get (Variables|Default|SetspawnTimerTentacle (+ DeltaSeconds (stale _output_get))))
                  (bind _outactors_6 (Actor|GetAllActorswithTag "Tentacle"))
                  (for (_array_element_6 _array_index_3) _outactors_6
                    (Utilities|Map|Add _members_2 _array_element_6 _array_index_3))
                  (if (== (Utilities|Map|Length _members_2) 0)
                    (if (Utilities|Array|ContainsItem _winner_3 "Creature")
                      (Utilities|Array|RemoveItem _winner_3 "Creature")
                      (goto _label))
                    (else
                      (Utilities|Map|Clear _members_2)
                      (Math|Float|CompareFloat _output_get 14.0
                        (:>
                          (bind _output_get_2 (Variables|Default|SetrandomLocation (Math|Vector|MakeVector (Math|Random|RandomFloatinRange -2e+03 2e+03) (Math|Random|RandomFloatinRange -2e+03 2e+03) -2.5e+02) :!label _label_3))
                          (Math|Float|CompareFloat (Math|Vector|Distance(Vector) "0, 0, 0" _output_get_2) 2.3e+03
                            (:>
                              (goto _label_3))
                            (:<
                              (Game|SpawnActorfromClass "/Game/Blueprints/TentacleBP.TentacleBP_C" (Math|Transform|MakeTransform _output_get_2 (Math|Rotator|MakeRotator 0.0 0.0 (Math|Random|RandomFloatinRange 0.0 3.6e+02)) "0.700000,0.700000,0.700000") "DontSpawnIfColliding" 0 0)
                              (Variables|Default|SetspawnTimerTentacle 0.0)
                              (Audio|PlaySound2D "/Game/Audio/Creature_create.Creature_create" 1.0 1.0 0.0 0 0))))))))))))
        (else
          (Utilities|Map|Clear _members_3)
          (goto _label_2))))))

(fn ConstructionScript)

(fn NewFunction0)
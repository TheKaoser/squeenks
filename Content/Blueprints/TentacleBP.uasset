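; Tentacle creature actor that automatically kills the nearest actor tagged NonTentacle, with animations, sounds and effects.
; Tick picks the closest target via a distance-keyed map, regrows the eye, then fires a short-lived ray and destroys non-busy SqueenkBP or BeastBP targets.
; A looping BeginPlay chain turns the tentacle toward its target, pausing while busy attacking.
; Setting the Death flag plays the death sequence and destroys the actor.
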(event EventBeginPlay
  (bind _focus (Variables|Default|Getfocus))
  (bind _tentacle (Variables|Default|GetTentacle))
  (bind _returnvalue (Transformation|GetWorldLocation _tentacle))
  (bind _rootcomponent (Variables|/Script/Engine.Actor|GetRootComponent _focus))
  (bind _returnvalue_2 (Transformation|GetWorldLocation _rootcomponent))
  (bind _returnvalue_3 (Math|Vector|GetUnitDirection(Vector) _returnvalue_2 _returnvalue))
  (Components|Animation|PlayAnimation _tentacle "/Game/Beings/Creature/Tentacle/tentacle_Anim_TentacleMesh_tentacle_full_cycle.tentacle_Anim_TentacleMesh_tentacle_full_cycle" false)
  (Utilities|FlowControl|Delay 0.2)
  (if (not (Variables|Default|Getempty)) :!label _label
    (if (Variables|Default|Getbusy)
      (Utilities|FlowControl|Delay 2.0)
      (goto _label)
      (else
        (Components|MoveComponentTo _tentacle _returnvalue (Math|Conversions|RotationFromXVector (Math|Vector|MakeVector (* (.y _returnvalue_3) 1.0) (* (.x _returnvalue_3) -1.0) 0.0)) false false 0.2 true)
        (goto _label)))))

(event EventTick
  (params (DeltaSeconds :type Float%20%28single-precision%29))
  (bind _possiblekills (Variables|Default|GetpossibleKills))
  (bind _eye (Variables|Default|Geteye))
  (bind _tentacle (Variables|Default|GetTentacle))
  (bind _returnvalue (Transformation|GetRelativeTransform _eye))
  (if (Variables|Default|Getdeath)
    (Variables|Default|Setdeath false)
    (Utilities|FlowControl|Delay 0.2)
    (Audio|PlaySound2D "/Game/Audio/Creature_death.Creature_death" 1.0 1.0 0.0 0 0)
    (Components|Animation|PlayAnimation _tentacle "/Game/Beings/Creature/Tentacle/tentacle_Anim_TentacleMesh_tentacle_death.tentacle_Anim_TentacleMesh_tentacle_death" false)
    (Transformation|SetRelativeTransform _eye (Math|Transform|MakeTransform (.location _returnvalue) (.rotation _returnvalue) "0.000000,0.000000,0.000000") false false)
    (Utilities|FlowControl|Delay 2.0)
    (Actor|DestroyActor)
    (elif (not (Variables|Default|Getbusy))
      (bind _outactors (Actor|GetAllActorswithTag "NonTentacle"))
      (for _array_element _outactors
        (Utilities|Map|Add _possiblekills (Math|Vector|Distance(Vector) (Transformation|GetWorldLocation _tentacle) (Transformation|GetWorldLocation (Variables|/Script/Engine.Actor|GetRootComponent _array_element))) _array_element)
        (if (< (Math|Vector|Distance(Vector) (Transformation|GetWorldLocation _tentacle) (Transformation|GetWorldLocation (Variables|/Script/Engine.Actor|GetRootComponent _array_element))) (Variables|Default|Getminimum))
          (Variables|Default|Setminimum (Math|Vector|Distance(Vector) (Transformation|GetWorldLocation _tentacle) (Transformation|GetWorldLocation (Variables|/Script/Engine.Actor|GetRootComponent _array_element))))))
      (if (== (Utilities|Map|Length _possiblekills) 0)
        (Variables|Default|Setempty true)
        (else
          (Variables|Default|Setempty false)
          (bind _output_get (Variables|Default|Setfocus (.Value (Utilities|Map|Find _possiblekills (Variables|Default|Getminimum)))))
          (Utilities|Map|Clear _possiblekills)
          (Variables|Default|Setminimum 1e+06)))
      (if (Audio|Components|Audio|IsPlaying _tentacle)
        _
        (else
          (Components|Animation|PlayAnimation _tentacle "/Game/Beings/Creature/Tentacle/tentacle_Anim_TentacleMesh_idle_pose.tentacle_Anim_TentacleMesh_idle_pose" false)))
      (if (Variables|Default|Getflag)
        (bind _assqueenk_bp (Utilities|Casting|CastToSqueenkBP _output_get)
          (:then
            (Utilities|IsValid _assqueenk_bp
              (:Is%20Valid
                (if (Variables|/Game/Blueprints/SqueenkBP.SqueenkBP_C|Getbusy _assqueenk_bp)
                  (Variables|Default|SettargetIsBusy true :!label _label)))))
          (:CastFailed
            (bind _asbeast_bp (Utilities|Casting|CastToBeastBP _output_get))
            (Utilities|IsValid _asbeast_bp
              (:Is%20Valid
                (if (Variables|/Game/Blueprints/BeastBP.BeastBP_C|Getbusy _asbeast_bp)
                  (goto _label)
                  (else
                    _))))))
        (if (Math|Boolean|ANDBoolean (not (Audio|Components|Audio|IsPlaying _eye)) (Variables|Default|Getflag) (not (Variables|Default|Getempty)) (not (Variables|Default|GettargetIsBusy)))
          (Components|Animation|PlayAnimation _tentacle "/Game/Beings/Creature/Tentacle/tentacle_Anim_TentacleMesh_tentacle_attack.tentacle_Anim_TentacleMesh_tentacle_attack" false)
          (Audio|PlaySound2D "/Game/Audio/Creature_attack.Creature_attack" 1.0 1.0 0.0 0 0)
          (bind _returnvalue_2 (Game|SpawnActorfromClass "/Game/Blueprints/CreaturetRayBP.CreaturetRayBP_C" (Math|Transform|MakeTransform (Transformation|GetWorldLocation _eye) "0, 0, 0" "1,1,1") "Undefined" 0 0))
          (Effects|Components|ParticleSystem|SetActorParameter (Variables|/Game/Blueprints/CreaturetRayBP.CreaturetRayBP_C|GetCreatureRay _returnvalue_2) "Target" (Variables|Default|Getfocus))
          (Actor|SetLifeSpan _returnvalue_2 0.2)
          (Variables|Default|Setbusy true)
          (bind _returnvalue_3 (Effects|SpawnEmitteratLocation "/Game/Effects/Death.Death" (Transformation|GetActorLocation (Variables|Default|Getfocus))))
          (bind _assqueenk_bp_2 (Utilities|Casting|CastToSqueenkBP (Variables|Default|Getfocus))
            (:then
              _)
            (:CastFailed
              _))
          (if (Utilities|IsValid _assqueenk_bp_2)
            (Effects|Components|ParticleSystem|SetColorParameter _returnvalue_3 "color" "(R=0.781250,G=0.159503,B=0.708507,A=1.000000)")
            (else
              (Effects|Components|ParticleSystem|SetColorParameter _returnvalue_3 "color" "(R=0.041667,G=0.021791,B=0.041134,A=1.000000)")))
          (Actor|DestroyActor (Variables|Default|Getfocus))
          (Audio|PlaySound2D "/Game/Audio/Death.Death" 1.0 1.0 0.25 0 0)
          (Variables|Default|Setfocus 0)
          (Transformation|SetRelativeTransform _eye (Math|Transform|MakeTransform (.location _returnvalue) (.rotation _returnvalue) "0.000000,0.000000,0.000000") false false)
          (Variables|Default|Setflag false)
          (Utilities|FlowControl|Delay 2.0)
          (Variables|Default|Setbusy false)
          (else
            (Variables|Default|SettargetIsBusy false)))
        (else
          (Variables|Default|Setflag true)
          (Components|Animation|PlayAnimation _eye "/Game/Beings/Creature/Eye/eye_Anim_Eye_Mesh_Increase.eye_Anim_Eye_Mesh_Increase" false)
          (Transformation|SetRelativeTransform _eye (Math|Transform|MakeTransform (.location _returnvalue) (.rotation _returnvalue) "0.700000,0.700000,0.700000") false false)
          (Utilities|FlowControl|Delay 2.0)
          (Variables|Default|Setembryo false))))))

(fn ConstructionScript)